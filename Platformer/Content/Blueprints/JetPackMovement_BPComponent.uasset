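; Actor component that gives the owning player a fuel-limited jetpack.
; While enabled and flying, Tick drains the remaining time and applies an upward force through the character movement component, resetting the recharge delay.
; When not flying or out of fuel, the delay counts down, scaled by the recharge rate, then fuel refills until it reaches capacity.
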(event `self.ReceiveBeginPlay`)

(event `self.ReceiveTick`
  (params (DeltaSeconds :type "Float (single-precision)"))
  (if (`self.Enable`)
    (if (`self.Fly`)
      (if (> (`self.RemaningTime`) 0.0)
        (set `self.RechargeDelayTimer` (`self.RechargeDelay`))
        (set `self.RemaningTime` (- (`self.RemaningTime`) DeltaSeconds))
        (`CharacterMovementComponent.AddForce` (`Character.CharacterMovement` (`self.OwningPlayer`)) (`KismetMathLibrary.MakeVector` 0.0 0.0 (`self.Force`)))
        (else
          (if (> (`self.RechargeDelayTimer`) 0.0) :!label _label
            (set `self.RechargeDelayTimer` (- (`self.RechargeDelayTimer`) (* (`self.RechargeRate`) DeltaSeconds)))
            (elif (not (>= (`self.RemaningTime`) (`self.Capacity`)))
              (set `self.RemaningTime` (+ (`self.RemaningTime`) (* (`self.RechargeRate`) DeltaSeconds)))))))
      (else
        (goto _label)))))