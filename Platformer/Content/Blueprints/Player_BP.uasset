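; Player character for a side-on shooter on the Y-Z plane, with sprint, crouch, jump, a jetpack and a grenade cannon.
; Each tick, a cursor trace sets facing, look angle, signed speed and projectile spawn rotation; while sprinting, facing follows movement instead.
; A Jetpack pickup enables the movement component, flown by pressing jump mid-air.
; Firing spends carried grenades; damage scales self-inflicted hits and triggers death, destroying attached actors and blocking input actions.
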(event `self.ReceiveBeginPlay`
  (bind (_returnvalue_x _returnvalue_y _returnvalue_z) (`KismetMathLibrary.BreakVector` (`self.K2_GetActorLocation`)))
  (set `/Game/Blueprints/JetPackMovement_BPComponent.OwningPlayer` self (`self.JetPackMovement_BPComponent`))
  (bind _returnvalue (`|CreateWidget` "/Game/Blueprints/UI/PlayerHUD.PlayerHUD_C"))
  (`UserWidget.AddToViewport` _returnvalue 0)
  (set `self.Health` (`self.MaxHealth`))
  (bind _returnvalue_2 (`|SpawnActorFromClass` "/Game/Blueprints/Weapons/BombCanon/GrenadeCanonVisual_BP.GrenadeCanonVisual_BP_C" (`KismetMathLibrary.MakeTransform` (0.0 0.0 0.0) (struct)) "AlwaysSpawn" "OverrideRootScale"))
  (`KismetArrayLibrary.Array_Add` (`self.ActorsToDestroyOnDeath`) _returnvalue_2)
  (`self.K2_AttachRootComponentTo` _returnvalue_2 (`self.Mesh`) "GunAttachPoint" "KeepRelativeOffset" true)
  (set `PlayerController.bShowMouseCursor` true (`GameplayStatics.GetPlayerController` 0))
  (`self.K2_SetActorLocation` (`KismetMathLibrary.MakeVector` 0.0 _returnvalue_y _returnvalue_z))
  (set `self.CurrentAmmo` (`self.GrenadeCanonGrenadsCarrying`)))

(event `self.ReceiveTick`
  (params (DeltaSeconds :type "Float (single-precision)"))
  (bind (_mouseposition_x _mouseposition_y _mouseposition_z) (`KismetMathLibrary.BreakVector` (`self.MousePosition`)))
  (bind (_returnvalue_x _returnvalue_y _returnvalue_z) (`KismetMathLibrary.BreakVector` (`SceneComponent.K2_GetComponentLocation` (`self.SpawnProjectileCenterPoint`))))
  (`|ExecutionSequence`
    (:`then_0`
      (`self.GetLookDirection`))
    (:`then_1`
      (`SceneComponent.K2_SetRelativeRotation` (`self.SpawnProjectileCenterPoint`) (`KismetMathLibrary.MakeRotator` (`KismetMathLibrary.DegAtan2` (- _mouseposition_y _returnvalue_y) (- _mouseposition_z _returnvalue_z))) false false))))

(event `InputAxis|MoveRight`
  (params (AxisValue :type "Float (single-precision)"))
  (bind _returnvalue (`NavMovementComponent.IsCrouching` (`self.CharacterMovement`)))
  (if (not (`self.Dead`))
    (if (`NavMovementComponent.IsFalling` (`self.CharacterMovement`))
      (`self.AddMovementInput` (0.0 1.0 0.0) AxisValue :!label _label)
      (elif (`self.Sprinting`)
        (if _returnvalue
          (goto _label)
          (elif (> AxisValue 0.3)
            (`self.AddMovementInput` (0.0 1.0 0.0) 1.0)
            (elif (< AxisValue -0.3)
              (`self.AddMovementInput` (0.0 -1.0 0.0) 1.0))))
        (elif _returnvalue
          (goto _label)
          (else
            (`self.AddMovementInput` (0.0 1.0 0.0) (* AxisValue (`self.RunSpeed`)))))))))

(event `InputAction|Jump`
  (params (Key :type "Key Structure" :default "AnyKey"))
  (bind _jetpackmovement_bpcomponent (`self.JetPackMovement_BPComponent`))
  (:`Pressed`
    (if (not (`self.Dead`))
      (if (not (`NavMovementComponent.IsFalling` (`self.CharacterMovement`)))
        (`self.Jump`)
        (else
          (set `/Game/Blueprints/JetPackMovement_BPComponent.Fly` true _jetpackmovement_bpcomponent)))))
  (:`Released`
    (set `/Game/Blueprints/JetPackMovement_BPComponent.Fly` false _jetpackmovement_bpcomponent)))

(event `InputAction|Crouch`
  (params (Key :type "Key Structure" :default "AnyKey"))
  (:`Pressed`
    (if (not (`self.Dead`))
      (if (not (`NavMovementComponent.IsFalling` (`self.CharacterMovement`)))
        (`self.Crouch`)
        (set `self.Sprinting` false))))
  (:`Released`
    (`self.UnCrouch`)))

(event `InputAction|Sprint`
  (params (Key :type "Key Structure" :default "AnyKey"))
  (:`Pressed`
    (if (not (`self.Dead`))
      (if (not (`NavMovementComponent.IsCrouching` (`self.CharacterMovement`)))
        (set `self.Sprinting` true))))
  (:`Released`
    (set `self.Sprinting` false)))

(event `Pick Up PickUp`
  (params (PickUp :type "/Game/Blueprints/PickUps/PickUp_BP Object Reference"))
  (if (`KismetStringLibrary.EqualEqual_StrStr` (`/Game/Blueprints/PickUps/PickUp_BP.PickUpItem` PickUp) "Jetpack")
    (set `/Game/Blueprints/JetPackMovement_BPComponent.Enable` true (`self.JetPackMovement_BPComponent`))))

(event `self.ReceiveActorBeginOverlap`
  (params (OtherActor :type "Actor Object Reference"))
  (bind _aspick_up_bp (cast `/Game/Blueprints/PickUps/PickUp_BP` OtherActor))
  (`self.Pick Up PickUp` _aspick_up_bp))

(event `InputAction|Fire`
  (params (Key :type "Key Structure" :default "AnyKey"))
  (:`Pressed`
    (if (and (not (`self.Sprinting`)) (not (`self.Dead`)))
      (if (> (`self.GrenadeCanonGrenadsCarrying`) 0)
        (bind _output_get (set `self.GrenadeCanonGrenadsCarrying` (- (`self.GrenadeCanonGrenadsCarrying`) 1)))
        (set `self.CurrentAmmo` _output_get)
        (`|SpawnActorFromClass` "/Game/Blueprints/Weapons/BombCanon/GrenadeCanonProjectile_BP.GrenadeCanonProjectile_BP_C" (`SceneComponent.K2_GetComponentToWorld` (`self.SpawnProjectileSpawnPoint`)) "Undefined" "OverrideRootScale")
        (switch `int` (`KismetMathLibrary.RandomIntegerInRange` 0)
          (:`0`
            (`GameplayStatics.PlaySoundAtLocation` "/Game/UniversalSoundFX/Sound_Effects/EXPLOSIONS/Short/EXPLOSION_Short_Bright_Kickback_stereo.EXPLOSION_Short_Bright_Kickback_stereo")))))))

(event `GetLookDirection`
  (bind (_returnvalue_x _returnvalue_y) (`KismetMathLibrary.BreakVector` (`self.K2_GetActorLocation`)))
  (bind _returnvalue (`self.GetInputAxisValue`))
  (bind _mesh (`self.Mesh`))
  (bind _mesh_2 (`self.Mesh`))
  (bind (_mouseposition_x _mouseposition_y _mouseposition_z) (`KismetMathLibrary.BreakVector` (`self.MousePosition`)))
  (bind _returnvalue_2 (> (`self.GetInputAxisValue`) 0.0))
  (bind (_returnvalue_x_2 _returnvalue_y_2 _returnvalue_z) (`KismetMathLibrary.BreakVector` (`SceneComponent.K2_GetComponentLocation` (`self.LookDirectionSource`))))
  (bind _returnvalue_3 (`KismetMathLibrary.VSize` (`MovementComponent.Velocity` (`self.CharacterMovement`))))
  (bind _returnvalue_4 (- _mouseposition_z _returnvalue_z))
  (bind _returnvalue_5 (- _mouseposition_y _returnvalue_y_2))
  (bind _returnvalue_6 (- 0.0 _returnvalue_3))
  (if (not (`self.Dead`))
    (bind _output_get (set `self.MousePosition` (`.ImpactPoint` (`GameplayStatics.BreakHitResult` (`PlayerController.GetHitResultUnderCursorByChannel` (`GameplayStatics.GetPlayerController` 0) "TraceTypeQuery3" true)))))
    (if (not (`self.Sprinting`))
      (if (> (.y _output_get) _returnvalue_y)
        (`SceneComponent.K2_SetRelativeRotation` _mesh (struct) false false)
        (if _returnvalue_2
          (set `self.CurrentSpeed` _returnvalue_3)
          (else
            (set `self.CurrentSpeed` _returnvalue_6)))
        (set `self.LookDiretion` (`KismetMathLibrary.DegAtan2` _returnvalue_4 _returnvalue_5))
        (else
          (`SceneComponent.K2_SetRelativeRotation` _mesh (struct :`Yaw` 180.0) false false)
          (if _returnvalue_2
            (set `self.CurrentSpeed` _returnvalue_6)
            (else
              (set `self.CurrentSpeed` _returnvalue_3)))
          (set `self.LookDiretion` (+ (`KismetMathLibrary.DegAtan2` _returnvalue_5 _returnvalue_4) 90.0))))
      (elif (> _returnvalue 0.1)
        (`SceneComponent.K2_SetRelativeRotation` _mesh_2 (struct) false false)
        (set `self.CurrentSpeed` (`KismetMathLibrary.VSize` (`MovementComponent.Velocity` (`self.CharacterMovement`))) :!label _label)
        (elif (< _returnvalue -0.1)
          (`SceneComponent.K2_SetRelativeRotation` _mesh_2 (struct :`Yaw` 180.0) false false)
          (goto _label))))))

(event `/Game/Blueprints/DamageInterface_BPIF.Damage`
  (params (Damage :type "Float (single-precision)") (DamageFromPlayer :type Boolean))
  (bind _returnvalue (`self.K2_GetActorLocation`))
  (bind _health (`self.Health`))
  (if DamageFromPlayer
    (set `self.Health` (- _health (* Damage (`self.SelfInFlictedDamage`))))
    (else
      (set `self.Health` (- _health Damage))))
  (switch `int` (`KismetMathLibrary.RandomIntegerInRange` 0 1)
    (:`0`
      (`GameplayStatics.PlaySoundAtLocation` "/Game/UniversalSoundFX/Sound_Effects/IMPACTS/Generic/IMPACT_Generic_07_mono.IMPACT_Generic_07_mono" _returnvalue))
    (:`1`
      (`GameplayStatics.PlaySoundAtLocation` "/Game/UniversalSoundFX/Sound_Effects/IMPACTS/Generic/IMPACT_Generic_09_mono.IMPACT_Generic_09_mono" _returnvalue)))
  (`self.CheckIfDead`))

(event `CheckIfDead`
  (if (<= (`self.Health`) 0.0)
    (`self.Die`)
    (else
      (set `self.Dead` false))))

(event `Die`
  (`self.K2_DestroyActor` (`self.ActorsToDestroyOnDeath`))
  (set `self.Dead` true))

(fn `UserConstructionScript`)