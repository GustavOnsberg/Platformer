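; Grenade cannon projectile that explodes on a hit, on a bounce, or after an auto-detonation delay.
; All three triggers share one blast path, with the timer run by a Delay on Tick.
; The blast spawns an explosion particle actor, sends full damage flagged as player-dealt to every actor overlapping the range collision, then destroys the projectile.
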(event `self.ReceiveBeginPlay`)

(event `self.ReceiveTick`
  (params (DeltaSeconds :type "Float (single-precision)"))
  (bind _overlappingactors (`PrimitiveComponent.GetOverlappingActors` (`self.RangeCollision`) null))
  (`KismetSystemLibrary.Delay` (`self.AutoBlowTime`))
  (`|SpawnActorFromClass` "/Game/Blueprints/Weapons/BombCanon/GrenadeCanonProjectileExplosionParticle_BP.GrenadeCanonProjectileExplosionParticle_BP_C" (`self.GetTransform`) "Undefined" "OverrideRootScale" :!label _label)
  (for _index (range (+ (`KismetArrayLibrary.Array_Length` _overlappingactors) 1))
    (message `/Game/Blueprints/DamageInterface_BPIF.Damage` (`KismetArrayLibrary.Array_Get` _overlappingactors _index) (`self.FullDamage`) true))
  (`self.K2_DestroyActor`))

(event `self.ReceiveActorBeginOverlap`
  (params (OtherActor :type "Actor Object Reference")))

(event `self.ProjectileMovement.OnProjectileBounce`
  (params (ImpactResult :type "HitResult Structure (by ref)") (ImpactVelocity :type "Vector Structure (by ref)"))
  (goto _label))

(event `self.ReceiveHit`
  (params (MyComp :type "PrimitiveComponent Object Reference") (Other :type "Actor Object Reference") (OtherComp :type "PrimitiveComponent Object Reference") (bSelfMoved :type Boolean) (HitLocation :type "Vector Structure") (HitNormal :type "Vector Structure") (NormalImpulse :type "Vector Structure") (Hit :type "HitResult Structure (by ref)"))
  (goto _label))

(fn `UserConstructionScript`
  (`parent.UserConstructionScript`))